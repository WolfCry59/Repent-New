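; Raising platform actor that shuttles back and forth along the spline of a referenced Path.
; After a random startup delay, one timeline drives it to the spline's end and a second, played in reverse, brings it back, looping with pauses.
; Each timeline's alpha maps to spline distance, setting location and rotation.
; A Cone component shows during the forward move and hides once the platform returns.
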(event Custom|Start_Moving
  ;[1 1 1] This plays a timeline of the Raising Platform
  (if (Variables|Default|GetIsAtBottom)
    (bind _alpha (Timeline|Timeline PlayFromStart)
      (:Update
        (Transformation|SetActorLocationAndRotation (.location (Spline|GetTransformatDistanceAlongSpline (Variables|/Game/Blueprints/BP_Path.BP_Path_C|GetSpline (Variables|Default|GetPath)) (Math|Float|Lerp 0.0 (Spline|GetSplineLength (Variables|/Game/Blueprints/BP_Path.BP_Path_C|GetSpline (Variables|Default|GetPath))) _alpha) "World" false)) (.rotation (Spline|GetTransformatDistanceAlongSpline (Variables|/Game/Blueprints/BP_Path.BP_Path_C|GetSpline (Variables|Default|GetPath)) (Math|Float|Lerp 0.0 (Spline|GetSplineLength (Variables|/Game/Blueprints/BP_Path.BP_Path_C|GetSpline (Variables|Default|GetPath))) _alpha) "World" false)))
        (Rendering|SetVisibility (Variables|Default|GetCone) true false))
      (:Finished
        (Variables|Default|SetIsAtBottom false)
        (Utilities|FlowControl|Delay 3.0)
        (CallFunction|StartReverse)))))

(event Custom|Start%20Reverse
  ;[1 1 1] This plays a reversed animation of the Raising Platform
  (if (not (Variables|Default|GetIsAtBottom))
    (bind _alpha (Timeline|Timeline_0 ReverseFromEnd)
      (:Update
        (Transformation|SetActorLocationAndRotation (.location (Spline|GetTransformatDistanceAlongSpline (Variables|/Game/Blueprints/BP_Path.BP_Path_C|GetSpline (Variables|Default|GetPath)) (Math|Float|Lerp 0.0 (Spline|GetSplineLength (Variables|/Game/Blueprints/BP_Path.BP_Path_C|GetSpline (Variables|Default|GetPath))) _alpha) "World" false)) (.rotation (Spline|GetTransformatDistanceAlongSpline (Variables|/Game/Blueprints/BP_Path.BP_Path_C|GetSpline (Variables|Default|GetPath)) (Math|Float|Lerp 0.0 (Spline|GetSplineLength (Variables|/Game/Blueprints/BP_Path.BP_Path_C|GetSpline (Variables|Default|GetPath))) _alpha) "World" false))))
      (:Finished
        (Variables|Default|SetIsAtBottom true)
        (Rendering|SetVisibility (Variables|Default|GetCone) false false)
        (Utilities|FlowControl|Delay 3.0)
        (CallFunction|StartMoving)))))

(event EventBeginPlay
  (Variables|Default|SetIsAtBottom true)
  (Utilities|FlowControl|Delay (Math|Random|RandomFloatinRange 3.0 5.0))
  (CallFunction|StartMoving))

(fn ConstructionScript)